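; Player character with a world-space cursor, level-specific UI and death on entering water.
; BeginPlay shows the main menu or the forest map's item toolbar and minimap, based on level name.
; Tick moves CursorToWorld to the surface under the mouse, aligned to its normal.
; EnterWater shows a one-time death widget, locks controller movement, freezes time dilation and switches to UI-only input.
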(event `self.ReceiveBeginPlay`
  (`parent.ReceiveBeginPlay`)
  (bind _returnvalue (`GameplayStatics.GetCurrentLevelName` true))
  (switch `string` _returnvalue
    (:`MainMenu_Map`
      (bind _returnvalue_2 (`|CreateWidget` "/Game/UI/Menu/WBP_MainMenu.WBP_MainMenu_C"))
      (`UserWidget.AddToViewport` _returnvalue_2 0))
    (:`Forest_Map`
      (bind _returnvalue_3 (`|CreateWidget` "/Game/UI/WBP_ItemToolbar.WBP_ItemToolbar_C"))
      (bind _output_get (set `self.ToolbarRef` _returnvalue_3))
      (`UserWidget.AddToViewport` _output_get 0)
      (bind _returnvalue_4 (`|CreateWidget` "/Game/UI/Minimap/WBP_Minimap.WBP_Minimap_C"))
      (bind _output_get_2 (set `self.MinimapRef` _returnvalue_4))
      (`UserWidget.AddToViewport` _output_get_2 0))))

(event `self.ReceiveTick`
  (params (DeltaSeconds :type "Float (single-precision)"))
  (bind (_bblockinghit _binitialoverlap _time _distance _location _impactpoint _normal _impactnormal) (`GameplayStatics.BreakHitResult` (`PlayerController.GetHitResultUnderCursorByChannel` (`GameplayStatics.GetPlayerController` 0) "TraceTypeQuery1" true)))
  ;[1 1 1] Update cursor position
  (`parent.ReceiveTick` DeltaSeconds)
  (`SceneComponent.K2_SetWorldLocationAndRotation` (`self.CursorToWorld`) _location (`KismetMathLibrary.MakeRotationFromAxes` _impactnormal) false false))

(fn `EnterWater`
  (bind _asbp_player_controller (cast `/Game/Player/BP_PlayerController` (`self.GetController`) :!pure true))
  (`/Engine/EditorBlueprintResources/StandardMacros.IsValid` (`self.Death`)
    (:`Is Not Valid`
      (bind _returnvalue (`|CreateWidget` "/Game/UI/Menu/WBP_Death.WBP_Death_C" null null "Water" "Wait 30 minutes after eating before trying to swim"))
      (set `self.Death` _returnvalue)
      (`UserWidget.AddToViewport` _returnvalue 0)
      (set `/Game/Player/BP_PlayerController.bMovementLocked` true _asbp_player_controller)
      (`GameplayStatics.SetGlobalTimeDilation` 0.0)
      (`WidgetBlueprintLibrary.SetInputMode_UIOnlyEx` _asbp_player_controller null))))

(fn `GetCenter`
  (returns (Center :type "Vector Structure"))
  (return (`self.K2_GetActorLocation`)))

(fn `GetGroundDistance`
  (returns (Distance :type "Float (double-precision)"))
  (return 200.0))

(fn `UserConstructionScript`)