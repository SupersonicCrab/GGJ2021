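; BP_Shrub is an obstacle that slows characters moving through its Box volume.
; On begin overlap, any BP_Character has MaxWalkSpeed set to a fraction of its MaxWalkSpeedCrouched, with BP_PlayerCharacter slowed less than other characters.
; On end overlap, MaxWalkSpeed is set to the full MaxWalkSpeedCrouched, so that property acts as the stored base speed.
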(event `self.Box.OnComponentBeginOverlap`
  (params (OverlappedComponent :type "PrimitiveComponent Object Reference") (OtherActor :type "Actor Object Reference") (OtherComp :type "PrimitiveComponent Object Reference") (OtherBodyIndex :type Integer) (bFromSweep :type Boolean) (SweepResult :type "HitResult Structure (by ref)"))
  (bind _asbp_character (cast `/Game/Character/BP_Character` OtherActor))
  (bind _asbp_player_character (cast `/Game/Player/BP_PlayerCharacter` OtherActor)
    (:`then`
      (bind _charactermovement (`Character.CharacterMovement` _asbp_player_character))
      (set `CharacterMovementComponent.MaxWalkSpeed` (/ (`CharacterMovementComponent.MaxWalkSpeedCrouched` _charactermovement) 2.0) _charactermovement))
    (:`CastFailed`
      (bind _charactermovement_2 (`Character.CharacterMovement` _asbp_character))
      (set `CharacterMovementComponent.MaxWalkSpeed` (/ (`CharacterMovementComponent.MaxWalkSpeedCrouched` _charactermovement_2) 4.0) _charactermovement_2))))

(event `self.Box.OnComponentEndOverlap`
  (params (OverlappedComponent :type "PrimitiveComponent Object Reference") (OtherActor :type "Actor Object Reference") (OtherComp :type "PrimitiveComponent Object Reference") (OtherBodyIndex :type Integer))
  (bind _asbp_character (cast `/Game/Character/BP_Character` OtherActor))
  (bind _charactermovement (`Character.CharacterMovement` _asbp_character))
  (set `CharacterMovementComponent.MaxWalkSpeed` (`CharacterMovementComponent.MaxWalkSpeedCrouched` _charactermovement) _charactermovement))

(fn `UserConstructionScript`
  (`parent.UserConstructionScript`))