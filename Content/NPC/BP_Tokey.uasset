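; BP_Tokey is an NPC character that favors rivers when navigating and moves much faster in water than out of it.
; On BeginPlay it sets its AI controller's default navigation filter to BP_PreferRiversFilter.
; Each Tick calls the parent, then switches the movement component's max walk speed based on the InWater flag, which this graph only reads.
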(event `self.ReceiveBeginPlay`
  (set `AIController.DefaultNavigationFilterClass` "/Game/NPC/BP_PreferRiversFilter.BP_PreferRiversFilter_C" (`AIBlueprintHelperLibrary.GetAIController` self)))

(event `self.ReceiveTick`
  (params (DeltaSeconds :type "Float (single-precision)"))
  (bind _charactermovement (`self.CharacterMovement`))
  (`parent.ReceiveTick` DeltaSeconds)
  (if (`self.bInWater`)
    (set `CharacterMovementComponent.MaxWalkSpeed` 600.0 _charactermovement)
    (else
      (set `CharacterMovementComponent.MaxWalkSpeed` 100.0 _charactermovement))))

(fn `UserConstructionScript`
  (`parent.UserConstructionScript`))