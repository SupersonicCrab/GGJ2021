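; Rusty is an NPC who turns hostile when the player interacts with him after retrieving every toolbar item; otherwise he uses the parent interaction.
; The trigger locks player movement, opens an enraged dialogue widget and sets global time dilation to zero before a short delay.
; OnEnraged then swaps his sprite, sets the Enraged flag that blocks further interaction, and sends his AI controller toward the player.
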(event `/Game/Player/BP_InteractInterface.InteractWithActor`
  (params (Player :type "/Game/Player/BP_PlayerCharacter Object Reference"))
  (if (not (`self.bEnraged`))
    (for _array_element (`/Game/UI/WBP_ItemToolbar.ItemRetrieved` (`/Game/Player/BP_PlayerCharacter.ToolbarRef` Player))
      (if (not _array_element)
        (break)))
    (if _array_element
      (set `/Game/Player/BP_PlayerController.bMovementLocked` true (cast `/Game/Player/BP_PlayerController` (`self.GetController` Player) :!pure true))
      (bind _returnvalue (`|CreateWidget` "/Game/UI/WBP_Dialogue.WBP_Dialogue_C" null (`self.NPCName`) (`self.EnragedIcon`) (`self.EnragedDialogue`)))
      (`UserWidget.AddToViewport` _returnvalue 0)
      (`GameplayStatics.SetGlobalTimeDilation` 0.0)
      (`KismetSystemLibrary.Delay` 1.5)
      (`self.OnEnraged`)
      (else
        (`parent.InteractWithActor` Player)))))

(fn `OnEnraged`
  (`PaperSpriteComponent.SetSprite` (`self.NPCSprite`) "/Game/Assets/Textures/NPCs/T_RustyEnraged_Sprite.T_RustyEnraged_Sprite")
  (set `self.bEnraged` true)
  (`AIController.MoveToActor` (`AIBlueprintHelperLibrary.GetAIController` self) (`GameplayStatics.GetPlayerCharacter` 0) 10.0 true true true null true))

(fn `UserConstructionScript`
  (`parent.UserConstructionScript`))