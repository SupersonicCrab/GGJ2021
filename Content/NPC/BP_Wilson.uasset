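; Wilson NPC character whose AI controller gets the BP_UseRivers navigation filter as default on BeginPlay, letting its pathfinding treat rivers differently.
; Each tick, after the parent's logic, the static mesh follows the capsule's XY at a fixed world height while moving, and returns to its relative offset below the capsule when stationary.
; GetGroundDistance always returns zero and EnterWater is empty.
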(event `self.ReceiveBeginPlay`
  (set `AIController.DefaultNavigationFilterClass` "/Game/NPC/BP_UseRivers.BP_UseRivers_C" (`AIBlueprintHelperLibrary.GetAIController` self)))

(event `self.ReceiveTick`
  (params (DeltaSeconds :type "Float (single-precision)"))
  (bind _staticmesh (`self.StaticMesh`))
  (bind (_returnvalue_x _returnvalue_y) (`KismetMathLibrary.BreakVector` (`SceneComponent.K2_GetComponentLocation` (`self.CapsuleComponent`))))
  (`parent.ReceiveTick` DeltaSeconds)
  (if (> (`KismetMathLibrary.VSize` (`MovementComponent.Velocity` (`self.CharacterMovement`))) 0.0)
    (`SceneComponent.K2_SetWorldLocation` _staticmesh (`KismetMathLibrary.MakeVector` _returnvalue_x _returnvalue_y 350.0) false false)
    (else
      (`SceneComponent.K2_SetRelativeLocation` _staticmesh (0.0 0.0 -87.999992) false false))))

(fn `EnterWater`)

(fn `GetGroundDistance`
  (returns (Distance :type "Float (double-precision)"))
  (return 0.0))

(fn `UserConstructionScript`
  (`parent.UserConstructionScript`))