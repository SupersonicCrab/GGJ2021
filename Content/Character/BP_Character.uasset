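; Base character Blueprint that adds a walking wobble, water detection and surface-based footstep sounds.
; Tick flags water when the mesh drops below a fixed height outside the main menu, and runs the Wobble timeline while moving.
; The timeline pitches the mesh and fires footsteps, choosing splash, bridge rock or grass sounds via a downward trace.
; EnterWater, GetCenter and GetGroundDistance are empty stubs, apparently for child classes.
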(event `self.ReceiveBeginPlay`
  (bind _charactermovement (`self.CharacterMovement`))
  (set `CharacterMovementComponent.MaxWalkSpeedCrouched` (`CharacterMovementComponent.MaxWalkSpeed` _charactermovement) _charactermovement))

(event `self.ReceiveTick`
  (params (DeltaSeconds :type "Float (single-precision)"))
  (bind _wobble (`self.Wobble`))
  (bind _mesh (`self.Mesh`))
  (bind (_returnvalue_x _returnvalue_y _returnvalue_z) (`KismetMathLibrary.BreakVector` (`SceneComponent.K2_GetComponentLocation` (`self.Mesh`))))
  (bind _returnvalue (`TimelineComponent.IsPlaying` _wobble))
  (bind (_relativerotation_roll _relativerotation_pitch _relativerotation_yaw) (`KismetMathLibrary.BreakRotator` (`SceneComponent.RelativeRotation` _mesh)))
  (bind _returnvalue_2 (`GameplayStatics.GetCurrentLevelName` true))
  (if (and (< _returnvalue_z 70.0) (not (`KismetStringLibrary.EqualEqual_StrStr` _returnvalue_2 "MainMenu_Map")))
    (`self.EnterWater`)
    (set `self.bInWater` true)
    (else
      (set `self.bInWater` false)))
  (if (!= (`KismetMathLibrary.VSize` (`MovementComponent.Velocity` (`self.CharacterMovement`))) 0.0)
    (if (not _returnvalue)
      (`TimelineComponent.PlayFromStart` _wobble))
    (elif _returnvalue
      (`TimelineComponent.Stop` _wobble)
      (`SceneComponent.K2_SetRelativeRotation` _mesh (`KismetMathLibrary.MakeRotator` _relativerotation_roll 0.0 _relativerotation_yaw) false false))))

(fn `EnterWater`)

(fn `GetCenter`
  (returns (Center :type "Vector Structure"))
  (return (0.0 0.0 0.0)))

(fn `GetGroundDistance`
  (returns (Distance :type "Float (double-precision)"))
  (return 0.0))

(fn `UserConstructionScript`)